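; ToolSpawner is a usable tool that plants fir saplings on landscape terrain, with a ghost preview of the placement.
; BeginPlay spawns a hidden, non-colliding marker with the sapling mesh, which is destroyed along with the tool.
; FindIntercection traces down from the holder's interaction capsule, treating only Landscape hits as valid.
; Tick uses it to move, show or hide and recolor the marker, while Use spawns the sapling at valid spots.
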(event `self.ReceiveDestroyed`
  (`self.K2_DestroyActor` (`self.SpawnMarker`)))

(event `self.ReceiveBeginPlay`
  (bind _returnvalue (`|SpawnActorFromClass` "/Script/Cosu.SpawnMark" (`KismetMathLibrary.MakeTransform` (0.0 0.0 0.0)) "AlwaysSpawn" "OverrideRootScale"))
  (bind _output_get (set `self.SpawnMarker` _returnvalue))
  (bind _staticmeshcomponent (`SpawnMark.StaticMeshComponent` _output_get))
  (`PrimitiveComponent.SetCollisionEnabled` _staticmeshcomponent "NoCollision")
  (`StaticMeshComponent.SetStaticMesh` _staticmeshcomponent "/Game/Meshes/Resources/Trees/SM_tree_fir_sapling.SM_tree_fir_sapling")
  (for (_ _array_index) (`MeshComponent.GetMaterials` _staticmeshcomponent)
    (`PrimitiveComponent.SetMaterial` _staticmeshcomponent _array_index "/Game/Meshes/Materials/Spawning/M_spawning_correct.M_spawning_correct"))
  (`self.SetActorHiddenInGame` (`self.SpawnMarker`) true))

(event `self.ReceiveTick`
  (params (DeltaSeconds :type "Float (single-precision)"))
  (bind _spawnmarker (`self.SpawnMarker`))
  (bind _staticmeshcomponent (`SpawnMark.StaticMeshComponent` _spawnmarker))
  (bind _returnvalue (not (`Actor.bHidden` (`self.SpawnMarker`))))
  (bind (_intercected _location _correctplace) (`self.FindIntercection`))
  (if (xor _intercected _returnvalue)
    (`self.SetActorHiddenInGame` (`self.SpawnMarker`) _returnvalue))
  (if _intercected
    (if _correctplace
      (set `self.SpawningCorrectness` "/Game/Meshes/Materials/Spawning/M_spawning_correct.M_spawning_correct")
      (else
        (set `self.SpawningCorrectness` "/Game/Meshes/Materials/Spawning/M_spawning_incorrect.M_spawning_incorrect")))
    (`self.K2_SetActorLocation` _spawnmarker _location false false)
    (for (_ _array_index) (`MeshComponent.GetMaterials` _staticmeshcomponent)
      (`PrimitiveComponent.SetMaterial` _staticmeshcomponent _array_index (`self.SpawningCorrectness`)))))

(event `self.Use`
  (bind (_intercected _location _correctplace) (`self.FindIntercection`))
  (if (and _intercected _correctplace)
    (`|SpawnActorFromClass` "/Game/Blueprints/Objects/Sapling_fir.Sapling_fir_C" (`KismetMathLibrary.MakeTransform` _location) "Undefined" "OverrideRootScale")))

(fn `FindIntercection`
  (returns (Intercected :type Boolean) (Location :type "Vector Structure") (CorrectPlace :type Boolean))
  (bind _interactioncollision (`/Game/Blueprints/Character/CosuCharacter.InteractionCollision` (`self.Holder`)))
  (bind _returnvalue (`SceneComponent.K2_GetComponentLocation` _interactioncollision))
  (bind (_outhit _returnvalue_2) (`KismetSystemLibrary.LineTraceSingleForObjects` :`Start` _returnvalue :`End` (- _returnvalue (`KismetMathLibrary.MakeVector` 0.0 0.0 (* (`CapsuleComponent.CapsuleHalfHeight` _interactioncollision) 1.5))) :`ObjectTypes` (`|MakeArray` "ObjectTypeQuery1" :!type "EObjectTypeQuery Enum") :`DrawDebugType` "ForOneFrame"))
  (if _returnvalue_2
    (bind (_bblockinghit _binitialoverlap _time _location _impactpoint _normal _impactnormal _physmat _hitactor) (`GameplayStatics.BreakHitResult` _outhit))
    (cast `Landscape` _hitactor
      (:`then`
        (return true _location true))
      (:`CastFailed`
        (return true _location false)))
    (else
      (return false _location false))))

(fn `UserConstructionScript`
  (`parent.UserConstructionScript`))