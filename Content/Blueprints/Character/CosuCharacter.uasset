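; Player character that holds one swappable tool and interacts with nearby actors.
; Slot inputs respawn the active tool (reselecting returns to hands), socketed to the first- or third-person mesh; the sapling input gives the spawner tool a test buildable.
; Attack uses the tool behind a duration lockout.
; Interact queries overlapping interface actors; timed interactions block move and look and show a progress widget until success or early-release failure.
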(event `Key|E`
  (params (Key :type "Key Structure" :default "AnyKey"))
  (:`Released`
    (bind _astool_spawner (cast `ToolSpawner` (`self.ActiveTool`)))
    (bind _output_get (set `ToolSpawner.bSnapIsOn` (not (stale _output_get)) _astool_spawner))))

(event `InputAction|Slot1`
  (params (Key :type "Key Structure" :default "AnyKey"))
  ;[1 1 1] QuickSlotsTools
  (:`Pressed`
    (`self.SetNewActiveTool` "/Game/Blueprints/Tools/ToolPickaxe.ToolPickaxe_C")))

(event `InputAction|Slot2`
  (params (Key :type "Key Structure" :default "AnyKey"))
  ;[1 1 1] QuickSlotsTools
  (:`Pressed`
    (`self.SetNewActiveTool` "/Game/Blueprints/Tools/ToolAxe.ToolAxe_C")))

(event `InputAction|Hands`
  (params (Key :type "Key Structure" :default "AnyKey"))
  ;[1 1 1] QuickSlotsTools
  (:`Pressed`
    (`self.SetNewActiveTool` "/Game/Blueprints/Tools/ToolHands.ToolHands_C")))

(event `InputAction|Sapling`
  (params (Key :type "Key Structure" :default "AnyKey"))
  ;[1 1 1] QuickSlotsTools
  (:`Pressed`
    (`self.SetNewActiveTool` "/Script/Cosu.ToolSpawner")
    (bind _astool_spawner (cast `ToolSpawner` (`self.ActiveTool`)))
    (bind _returnvalue (`|SpawnActorFromClass` "/Game/Blueprints/Objects/Buildable/BluildableSocketTest.BluildableSocketTest_C" (`KismetMathLibrary.MakeTransform` (0.0 0.0 0.0)) "AlwaysSpawn" "OverrideRootScale" self self))
    (`ToolSpawner.SetBuildable` _astool_spawner _returnvalue)
    (set `ToolSpawner.SnapDistance` 300.0 _astool_spawner)))

(event `self.ReceiveBeginPlay`
  (`parent.ReceiveBeginPlay`)
  (`self.SetNewActiveTool` "/Game/Blueprints/Tools/ToolHands.ToolHands_C")
  (`self.SetDurableInteractionTimerEnabled` false))

(event `self.OnCameraSwitched`
  (`self.AttachTool`))

(event `InputAction|Attack`
  (params (Key :type "Key Structure" :default "AnyKey"))
  (:`Pressed`
    (if (not (`self.IsAttacking`))
      (set `self.IsAttacking` true)
      (`/Game/Blueprints/Tools/ToolBase_BP.Use` (`self.ActiveTool`))
      (`KismetSystemLibrary.Delay` (`self.AttackDuration`))
      (set `self.IsAttacking` false))))

(event `CallInteractionSuccess`
  (message `InteractInterface.InteractionSuccess` (`self.InteractingWith`) self)
  (`self.FinishInteraction`))

(event `InputAction|Interact`
  (params (Key :type "Key Structure" :default "AnyKey"))
  (bind _interactingwith (`self.InteractingWith`))
  (:`Pressed`
    (bind _overlappingactors (`self.GetInteractableActors` null))
    (for _array_element _overlappingactors
      (if (`KismetSystemLibrary.DoesImplementInterface` _array_element "/Script/Cosu.InteractInterface")
        (bind (_outduration _returnvalue) (message `InteractInterface.RequestInteraction` _array_element self))
        (if _returnvalue
          (if (> _outduration 0.0)
            (set `self.InteractingWith` _array_element)
            (`self.BlockMovement`)
            (bind _returnvalue_2 (`KismetSystemLibrary.K2_SetTimerDelegate` (delegate `CallInteractionSuccess`) _outduration))
            (set `self.InteractionTimer` _returnvalue_2)
            (`self.SetDurableInteractionTimerEnabled` true)
            (break)
            (else
              (break)))))))
  (:`Released`
    (`/Engine/EditorBlueprintResources/StandardMacros.IsValid` _interactingwith
      (:`Is Valid`
        (message `InteractInterface.InteractionFailure` _interactingwith self)
        (`self.FinishInteraction`)))))

(event `FinishInteraction`
  (`self.UnblockMovement`)
  (set `self.InteractingWith` null)
  (`self.SetDurableInteractionTimerEnabled` false))

(event `BlockMovement`
  (bind _returnvalue (`self.GetController`))
  (`Controller.SetIgnoreMoveInput` _returnvalue true)
  (`Controller.SetIgnoreLookInput` _returnvalue true))

(event `UnblockMovement`
  (bind _returnvalue (`self.GetController`))
  (`Controller.SetIgnoreMoveInput` _returnvalue false)
  (`Controller.SetIgnoreLookInput` _returnvalue false))

(event `SetDurableInteractionTimerEnabled`
  (params (Enabled :type Boolean))
  (bind _durableinteractionprogress (`self.DurableInteractionProgress`))
  (bind _asw_durable_interaction_progress (cast `/Game/Blueprints/UI/Interaction/W_DurableInteractionProgress` (`WidgetComponent.GetUserWidgetObject` _durableinteractionprogress)))
  (`Widget.SetIsEnabled` _asw_durable_interaction_progress Enabled)
  (`SceneComponent.SetVisibility` _durableinteractionprogress Enabled false)
  (if Enabled
    (set `/Game/Blueprints/UI/Interaction/W_DurableInteractionProgress.InteractionTimer` (`self.InteractionTimer`) _asw_durable_interaction_progress)
    (`SceneComponent.K2_SetWorldLocation` (`self.DurableInteractionProgress`) (+ (`self.K2_GetActorLocation` (`self.InteractingWith`)) (0.0 0.0 100.0)) false false)))

(fn `AttachTool`
  (locals (MeshToAttachTo :type "SkeletalMeshComponent Object Reference"))
  (if (`self.IsInThirdPersonView`)
    (set `local.MeshToAttachTo` (`self.Mesh`))
    (else
      (set `local.MeshToAttachTo` (`self.FirstPersonMesh`))))
  (`self.K2_AttachToComponent` (`self.ActiveTool`) (`local.MeshToAttachTo`) "hand_rSocket" "SnapToTarget" "KeepRelative" "KeepRelative" true))

(fn `GetInteractableActors`
  (params (ClassFilter :type "Actor Class Reference"))
  (returns (OverlappingActors :type "Array of Actor Object Reference"))
  (return (`PrimitiveComponent.GetOverlappingActors` (`self.InteractionCollision`) ClassFilter)))

(fn `SetNewActiveTool`
  (params (NewTool :type "ToolBase Class Reference"))
  (bind _activetool (`self.ActiveTool`))
  (if (== NewTool (`GameplayStatics.GetObjectClass` (`self.ActiveTool`)))
    (if (!= (`GameplayStatics.GetObjectClass` (`self.ActiveTool`)) "/Game/Blueprints/Tools/ToolHands.ToolHands_C")
      (`self.SetNewActiveTool` "/Game/Blueprints/Tools/ToolHands.ToolHands_C"))
    (else
      (`/Engine/EditorBlueprintResources/StandardMacros.IsValid` _activetool
        (:`Is Valid`
          (`self.K2_DestroyActor` _activetool))
        (:`Is Not Valid`
          _))
      (bind _returnvalue (`|SpawnActorFromClass` NewTool (`KismetMathLibrary.MakeTransform` (0.0 0.0 0.0)) "Undefined" "OverrideRootScale" null self))
      (set `self.ActiveTool` _returnvalue)
      (set `/Game/Blueprints/Tools/ToolBase_BP.Holder` self (`self.ActiveTool`))
      (`self.AttachTool`))))

(fn `UserConstructionScript`
  (`parent.UserConstructionScript`))