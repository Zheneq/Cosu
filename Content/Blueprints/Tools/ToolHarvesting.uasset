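; ToolHarvesting is a tool Blueprint that lets its holder harvest nearby harvestable objects when used.
; On Use, it gathers HarvestableBase actors overlapping the holder's interaction collision and calls Harvest on each, passing the holder and itself.
; The loop stops at the first successful harvest, so each use harvests at most one object.
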(event `self.Use`
  (bind _overlappingactors (`PrimitiveComponent.GetOverlappingActors` (`/Game/Blueprints/Character/CosuCharacter.InteractionCollision` (`self.Holder`)) "/Game/Blueprints/Objects/Harvestable/HarvestableBase.HarvestableBase_C"))
  (if (> (`KismetArrayLibrary.Array_Length` _overlappingactors) 0)
    (for _array_element _overlappingactors
      (bind _asharvestable_base (cast `/Game/Blueprints/Objects/Harvestable/HarvestableBase` _array_element))
      (bind _washarvested (`/Game/Blueprints/Objects/Harvestable/HarvestableBase.Harvest` _asharvestable_base (`self.Holder`) self))
      (if _washarvested
        (break)))))

(fn `UserConstructionScript`
  (`parent.UserConstructionScript`))